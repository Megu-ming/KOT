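; Potion pickup actor that puts its potion type into the player controller's first item slot, then destroys itself and plays a sound.
; ItemSetup fills the pickup widget's label with the item name, colored by the Health, Mana or DeathsDoor enum.
; The construction script is empty; disconnected per-potion branches would set mesh, light color, text, collision radius and rotation speed through a dynamic material instance.
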(fn `ItemSetup`
  (bind _aswb_hud_pickup (cast `/Game/Blueprints/WidgetBP/WB_HUD_Pickup` (`WidgetComponent.GetUserWidgetObject` (`self.Widget`))))
  (bind _textblocklabel (`/Game/Blueprints/WidgetBP/WB_HUD_Pickup.TextBlockLabel` _aswb_hud_pickup))
  (`TextBlock.SetText` _textblocklabel (`self.ItemTextName`))
  (`TextBlock.SetColorAndOpacity` _textblocklabel (make `SlateColor` (select `/Game/Items/Pickups/PotionPickups/PotionList` (`self.PotionList`) :`NewEnumerator0` (struct :`G` 1.0 :`A` 1.0) :`NewEnumerator1` (struct :`G` 1.0 :`B` 1.0 :`A` 1.0) :`NewEnumerator2` (struct :`R` 1.0 :`G` 0.25 :`A` 1.0) :!type "LinearColor Structure"))))

(fn `UserConstructionScript`)